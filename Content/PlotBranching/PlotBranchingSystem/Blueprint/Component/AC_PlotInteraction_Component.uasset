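; Plot interaction component that runs click-advanced, branching dialogue through a UI_Dialog widget it creates on BeginPlay.
; Plot assets supply lines, options and settings, and each line waits a length-scaled Delay before advancing is allowed.
; A choice panel opens mid-plot or at the end; choices load a branch asset or end the plot and enable the next trigger box's guidance.
; E messages the interacting actor, which also receives a sequence message as lines finish.
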(event Custom|AC_Event_Plote%20Start
  (params (Restrict%20player%20movement :type Boolean) (Restrict%20player%20perspective :type Boolean) (Plot_Data :type PDA%20Plot%20Data%20Object%20Reference))
  (bind _line (Variables|交互部分|GetLine))
  (bind _current_number (Variables|交互部分|GetCurrent%20number))
  (bind _output (Utilities|Array|Get(acopy) _line _current_number))
  ;[1 0.2741 0] 开始触发
  ;[0 0.7967 1] 关闭交互提示
  (Default|UIEventInteractivePrompts (Variables|Default|GetUI_Dialog) "Collapsed")
  (CallFunction|GatData Plot_Data)
  ;[0 0.7967 1] 开启对话框
  (Default|UIEventDisplayDialog (Variables|Default|GetUI_Dialog) "Visible")
  ;[1 0.2741 0] 将资产内容传输给UI
  ;;[0 0.7967 1] 把台词设置给UI
  (Default|UIEventSetDialogueText (Variables|Default|GetUI_Dialog) _output)
  (Utilities|FlowControl|Delay (* (Utilities|String|Len (Utilities|String|ToString(Text) _output)) (Variables|交互部分|GetBasic%20line%20dwell%20time)))
  (if (Variables|条件部分|GetSelect%20at%20end)
    ;;[0 0.7967 1] 开启提示
    (Default|UIEventSetPrompts (Variables|Default|GetUI_Dialog) "Visible" :!label _label)
    ;;[0 0.7967 1] 设置当前台词已经结束
    (Variables|条件部分|SetDialogue%20ends true)
    ;;[0 0.7967 1] 计算下句台词编号
    (Math|Integer|IncrementInt (Variables|交互部分|GetCurrent%20number)
      (:%20%20
        (Class|BPIInteractive|PlaySequence(Message) (Variables|Default|GetInteracting%20Actor))))
    (elif (== (Variables|交互部分|GetCurrent%20number) (Variables|交互部分|GetTrigger%20Selection%20Number))
      (CallFunction|ACEventSetSelectionEnable "Visible")
      (else
        (goto _label)))))

(event Custom|AC_Event_Plot%20End
  ;[0 0.7967 1] 关闭对话框
  (Default|UIEventDisplayDialog (Variables|Default|GetUI_Dialog) "Collapsed")
  (Default|UIEventSetPrompts (Variables|Default|GetUI_Dialog) "Collapsed")
  (Default|UIEventShowBranches (Variables|Default|GetUI_Dialog) "Collapsed")
  (Variables|交互部分|SetCurrent%20number 0)
  (Utilities|Array|Clear (Variables|交互部分|GetLine))
  (Variables|条件部分|SetIn%20the%20plot false)
  (Variables|条件部分|SetGet%20Target false))

(event Custom|AC_Event_Injecting%20Branch%20Plot
  (params (self2 :type PDA%20Plot%20Data%20Object%20Reference))
  ;[1 0.2741 0] 选择分支剧情
  ;;[1 0.2741 0] 在选择结束后结束交互
  (if (not (Variables|Default|GetSelect%20End%20Exit))
    (CallFunction|GatData self2)
    (Variables|交互部分|SetCurrent%20number 0)
    (Default|UIEventShowBranches (Variables|Default|GetUI_Dialog) "Collapsed")
    (Default|UIEventDisplayDialog (Variables|Default|GetUI_Dialog) "Visible")
    ;[1 0.2741 0] 将资产内容传输给UI
    ;;[0 0.7967 1] 把台词设置给UI
    (Default|UIEventSetDialogueText (Variables|Default|GetUI_Dialog) (Utilities|Array|Get(acopy) (Variables|交互部分|GetLine) (Variables|交互部分|GetCurrent%20number)))
    (Utilities|FlowControl|Delay (* (Utilities|String|Len (Utilities|String|ToString(Text) (Utilities|Array|Get(acopy) (Variables|交互部分|GetLine) (Variables|交互部分|GetCurrent%20number)))) (Variables|交互部分|GetBasic%20line%20dwell%20time)))
    (if (Variables|条件部分|GetSelect%20at%20end)
      ;;[0 0.7967 1] 开启提示
      (Default|UIEventSetPrompts (Variables|Default|GetUI_Dialog) "Visible" :!label _label)
      ;;[0 0.7967 1] 设置当前台词已经结束
      (Variables|条件部分|SetDialogue%20ends true)
      ;;[0 0.7967 1] 计算下句台词编号
      (Math|Integer|IncrementInt (Variables|交互部分|GetCurrent%20number)
        (:%20%20
          (Class|BPIInteractive|PlaySequence(Message) (Variables|Default|GetInteracting%20Actor))))
      (elif (== (Variables|交互部分|GetCurrent%20number) (Variables|交互部分|GetTrigger%20Selection%20Number))
        (CallFunction|ACEventSetSelectionEnable "Visible")
        (else
          (goto _label))))
    (else
      (Utilities|FlowControl|Sequence
        (:then_0
          (CallFunction|ACEventPlotEnd))
        (:then_1
          (Utilities|FlowControl|Delay 0.1)
          (CallFunction|ACEventEnableGuidance (Variables|Default|GetNext%20Trigger%20Box)))))))

(event Custom|AC_Event_Set%20Selection%20Enable
  (params (InVisibility :type ESlateVisibility%20Enum :default "Visible"))
  (bind _returnvalue (Game|GetPlayerController 0))
  ;[1 0.2741 0] 设置显示选择面板
  (Default|UIEventShowBranches (Variables|Default|GetUI_Dialog) InVisibility)
  (switch Utilities|FlowControl|Switch|SwitchonESlateVisibility InVisibility
    (:Visible
      (Default|UIEventDisplayDialog (Variables|Default|GetUI_Dialog) "Collapsed")
      (Variables|/Script/Engine.PlayerController|SetbShowMouseCursor _returnvalue true))
    (:Collapsed
      (Default|UIEventDisplayDialog (Variables|Default|GetUI_Dialog) "Visible")
      (Variables|/Script/Engine.PlayerController|SetbShowMouseCursor _returnvalue (Variables|Default|GetShow%20Mouse)))))

(event Custom|AC_Event_Enable%20Guidance
  (params (Next%20Trigger%20Box :type BP%20Plot%20Trigger%20Box%20Base%20Class%20Object%20Reference))
  (Default|EventOpenGuidance Next%20Trigger%20Box)
  (Default|EventSetEnableTrigger Next%20Trigger%20Box "QueryOnly"))

(event EventBeginPlay
  ;[0 0.7967 1] 在开始时设置UI
  (bind _returnvalue (UserInterface|CreateWidget "/Game/PlotBranching/PlotBranchingSystem/UI/UI_Dialog.UI_Dialog_C" (Game|GetPlayerController 0)))
  (UserInterface|Viewport|AddtoViewport _returnvalue 0)
  (bind _output_get (Variables|Default|SetUI_Dialog _returnvalue))
  (Default|UIEventGetComponent _output_get self))

(event EventGetInteractingActor
  (params (Actor :type Actor%20Object%20Reference))
  ;[1 0.2741 0] 物体交互部分
  (Variables|Default|SetInteracting%20Actor Actor)
  ;;[0 0.7967 1] 开启交互提示
  (Default|UIEventInteractivePrompts (Variables|Default|GetUI_Dialog) "Visible"))

(event Input|MouseEvents|LeftMouseButton
  (params (Key :type Key%20Structure))
  (bind _line (Variables|交互部分|GetLine))
  (bind _current_number (Variables|交互部分|GetCurrent%20number))
  (bind _output (Utilities|Array|Get(acopy) _line _current_number))
  ;[1 0.2741 0] 这里可以改成你们的交互按键
  (:Pressed
    ;[0 0.7967 1] 判断是否已经触发剧情
    (if (Variables|条件部分|GetIn%20the%20plot)
      ;[0 0.7967 1] 判断是否台词已经说完
      (if (not (== (Variables|交互部分|GetCurrent%20number) (Utilities|Array|Length (Variables|交互部分|GetLine))))
        ;[0 0.7967 1] 当前对话是否结束
        (if (Variables|条件部分|GetDialogue%20ends)
          (Default|UIEventSetPrompts (Variables|Default|GetUI_Dialog) "Collapsed")
          (Variables|条件部分|SetDialogue%20ends false)
          ;[1 0.2741 0] 将资产内容传输给UI
          ;;[0 0.7967 1] 把台词设置给UI
          (Default|UIEventSetDialogueText (Variables|Default|GetUI_Dialog) _output)
          (Utilities|FlowControl|Delay (* (Utilities|String|Len (Utilities|String|ToString(Text) _output)) (Variables|交互部分|GetBasic%20line%20dwell%20time)))
          (if (Variables|条件部分|GetSelect%20at%20end)
            ;;[0 0.7967 1] 开启提示
            (Default|UIEventSetPrompts (Variables|Default|GetUI_Dialog) "Visible" :!label _label)
            ;;[0 0.7967 1] 设置当前台词已经结束
            (Variables|条件部分|SetDialogue%20ends true)
            ;;[0 0.7967 1] 计算下句台词编号
            (Math|Integer|IncrementInt (Variables|交互部分|GetCurrent%20number)
              (:%20%20
                (Class|BPIInteractive|PlaySequence(Message) (Variables|Default|GetInteracting%20Actor))))
            (elif (== (Variables|交互部分|GetCurrent%20number) (Variables|交互部分|GetTrigger%20Selection%20Number))
              (CallFunction|ACEventSetSelectionEnable "Visible")
              (else
                (goto _label)))))
        (else
          ;[0 0.7967 1] 判断是否在对话结束时跳出选项界面
          (if (Variables|条件部分|GetSelect%20at%20end)
            (CallFunction|ACEventSetSelectionEnable "Visible")
            (else
              (CallFunction|ACEventPlotEnd))))))))

(event Input|KeyboardEvents|E
  (params (Key :type Key%20Structure))
  ;[1 0.2741 0] 物体交互部分
  ;;[0 0.7967 1] 这里改成你自己的按键
  (:Pressed
    (Class|BPIInteractive|Interactive(Message) (Variables|Default|GetInteracting%20Actor))))

(fn GatData
  (params (self2 :type PDA%20Plot%20Data%20Object%20Reference))
  (Utilities|IsValid self2
    (:Is%20Valid
      (bind _output_get (Variables|Default|SetPlpotData self2))
      (Utilities|FlowControl|Sequence
        (:then_0
          (Variables|交互部分|SetLine (Variables|/Game/PlotBranching/PlotBranchingSystem/Data/PDA_Plot_Data.PDA_Plot_Data_C|GetLine _output_get))
          (Variables|交互部分|SetTrigger%20Selection%20Number (- (Variables|/Game/PlotBranching/PlotBranchingSystem/Data/PDA_Plot_Data.PDA_Plot_Data_C|GetTrigger%20selection%20number _output_get) 1)))
        (:then_1
          (Default|UIEventGetBranchAssets (Variables|Default|GetUI_Dialog) (Variables|/Game/PlotBranching/PlotBranchingSystem/Data/PDA_Plot_Data.PDA_Plot_Data_C|GetOption%201%20-%20Plot%20Triggering%20Assets _output_get) (Variables|/Game/PlotBranching/PlotBranchingSystem/Data/PDA_Plot_Data.PDA_Plot_Data_C|GetOption%202%20-%20Plot%20Triggering%20Assets _output_get) (Variables|/Game/PlotBranching/PlotBranchingSystem/Data/PDA_Plot_Data.PDA_Plot_Data_C|GetOption%201-%20Answer _output_get) (Variables|/Game/PlotBranching/PlotBranchingSystem/Data/PDA_Plot_Data.PDA_Plot_Data_C|GetOption%202-%20Answer _output_get) (Variables|/Game/PlotBranching/PlotBranchingSystem/Data/PDA_Plot_Data.PDA_Plot_Data_C|GetQuestion%20Text _output_get)))
        (:then_2
          (bind _output_get_2 (Variables|Default|SetShow%20Mouse (Variables|/Game/PlotBranching/PlotBranchingSystem/Data/PDA_Plot_Data.PDA_Plot_Data_C|GetShow%20Mouse _output_get)))
          (Variables|/Script/Engine.PlayerController|SetbShowMouseCursor (Game|GetPlayerController 0) _output_get_2)
          (Variables|条件部分|SetSelect%20at%20end (Variables|/Game/PlotBranching/PlotBranchingSystem/Data/PDA_Plot_Data.PDA_Plot_Data_C|GetIs%20the%20selection%20triggered%20at%20the%20end _output_get))
          (Variables|Default|SetSelect%20End%20Exit (Variables|/Game/PlotBranching/PlotBranchingSystem/Data/PDA_Plot_Data.PDA_Plot_Data_C|GetEnd%20conversation%20after%20selection _output_get)))))
    (:Is%20Not%20Valid
      (return))))