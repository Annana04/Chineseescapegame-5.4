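; Plot control center for a branching plot system that links plot data to the trigger boxes of its two options.
; Each SetTrigger entry pairs a PlotData with two option trigger boxes, whose references are copied into that PlotData.
; The same copy loop runs in the Construction Script and again on BeginPlay.
; Tick prints debug text from the TextRender of both boxes in the entry at index 1.
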(event EventBeginPlay
  (for _array_element (Variables|Default|GetSet%20Trigger)
    (Variables|/Game/PlotBranching/PlotBranchingSystem/Data/PDA_Plot_Data.PDA_Plot_Data_C|SetOption%201%20-%20PlotTriggerBox (.Plot_Data (Utilities|Struct|BreakUDS_DataNaxtTrigger _array_element)) (.Option1-PlotTriggerBox (Utilities|Struct|BreakUDS_DataNaxtTrigger _array_element)))
    (Variables|/Game/PlotBranching/PlotBranchingSystem/Data/PDA_Plot_Data.PDA_Plot_Data_C|SetOption%202%20-%20PlotTriggerBox (.Plot_Data (Utilities|Struct|BreakUDS_DataNaxtTrigger _array_element)) (.Option2-PlotTriggerBox (Utilities|Struct|BreakUDS_DataNaxtTrigger _array_element)))))

(event EventTick
  (params (DeltaSeconds :type Float%20%28single-precision%29))
  (bind _set_trigger (Variables|Default|GetSet%20Trigger))
  (bind _output (Utilities|Array|Get(acopy) _set_trigger 1))
  (bind (_plot_data _option1_plottriggerbox _option2_plottriggerbox) (Utilities|Struct|BreakUDS_DataNaxtTrigger _output))
  (Development|PrintText (Utilities|Text|ToText(String) (Utilities|String|Append (Utilities|String|ToString(Text) (Variables|/Script/Engine.TextRenderComponent|GetText (Variables|/Game/PlotBranching/PlotBranchingSystem/Blueprint/BP_PlotTriggerBox_BaseClass.BP_PlotTriggerBox_BaseClass_C|GetTextRender _option1_plottriggerbox))) "                   " (Utilities|String|ToString(Text) (Variables|/Script/Engine.TextRenderComponent|GetText (Variables|/Game/PlotBranching/PlotBranchingSystem/Blueprint/BP_PlotTriggerBox_BaseClass.BP_PlotTriggerBox_BaseClass_C|GetTextRender _option2_plottriggerbox))))) true true "(R=0.000000,G=0.660000,B=1.000000,A=1.000000)" 0.0))

(fn ConstructionScript
  (for _array_element (Variables|Default|GetSet%20Trigger)
    (Variables|/Game/PlotBranching/PlotBranchingSystem/Data/PDA_Plot_Data.PDA_Plot_Data_C|SetOption%201%20-%20PlotTriggerBox (.Plot_Data (Utilities|Struct|BreakUDS_DataNaxtTrigger _array_element)) (.Option1-PlotTriggerBox (Utilities|Struct|BreakUDS_DataNaxtTrigger _array_element)))
    (Variables|/Game/PlotBranching/PlotBranchingSystem/Data/PDA_Plot_Data.PDA_Plot_Data_C|SetOption%202%20-%20PlotTriggerBox (.Plot_Data (Utilities|Struct|BreakUDS_DataNaxtTrigger _array_element)) (.Option2-PlotTriggerBox (Utilities|Struct|BreakUDS_DataNaxtTrigger _array_element)))))