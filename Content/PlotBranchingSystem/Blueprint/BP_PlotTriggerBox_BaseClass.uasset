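; Base trigger box actor for the plot branching system that starts a story segment for the player.
; On overlap it either starts immediately, registers for interaction, or checks a target condition, then hands PlotData and movement/view restrictions to the player's plot interaction component.
; It also manages a guidance widget, can turn the player toward a look-at actor, and plays indexed transition sequences.
; The construction script applies text, collision and box scale, and keeps trigger and interaction modes exclusive.
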(event OnComponentBeginOverlap(Box)
  (params (OverlappedComponent :type Primitive%20Component%20Object%20Reference) (OtherActor :type Actor%20Object%20Reference) (OtherComp :type Primitive%20Component%20Object%20Reference) (OtherBodyIndex :type Integer) (bFromSweep :type Boolean) (SweepResult :type Hit%20Result%20Structure%20%28by%20ref%29))
  (Utilities|FlowControl|DoOnce false
    (:Completed
      (if (== OtherActor (Variables|Default|GetPlayer))
        (Variables|Default|SetEnter%20trigger true)
        ;[0 0.7967 1] 使用触发器触发
        (if (Variables|条件|GetUsing%20triggers%20)
          (if (Variables|条件|GetDoOnce)
            (Utilities|FlowControl|DoOnce false
              (:Completed
                _)))
          (Variables|/Game/PlotBranchingSystem/Blueprint/Component/AC_PlotInteraction_Component.AC_PlotInteraction_Component_C|SetIn%20the%20plot (Variables|Default|Get%20Plot%20Interaction) true)
          (CallFunction|TriggerthePlot (Variables|Default|GetPlot_Data) :!label _label)
          (CallFunction|EventCloseGuidance)
          (Utilities|IsValid (Variables|条件|Getlook%20at%20actor)
            (:Is%20Valid
              (Transformation|SetActorRotation (Variables|Default|GetPlayer) (Math|Rotator|MakeRotator 0.0 0.0 (.yaw (Math|Rotator|FindLookatRotation (Transformation|GetActorLocation (Variables|Default|GetPlayer)) (Transformation|GetActorLocation (Variables|条件|Getlook%20at%20actor))))))))
          (else
            ;[0 0.7967 1] 使用交互触发
            (if (Variables|条件|GetFor%20interactive%20objects)
              (Class|BPIInteractive|GetInteractingActor(Message) (Variables|Default|Get%20Plot%20Interaction) self)
              (else
                (if (Variables|条件|GetDoOnce)
                  (Utilities|FlowControl|DoOnce false
                    (:Completed
                      _)))
                ;[0 0.7967 1] 判断是否达到目标(条件触发)
                (if (Variables|/Game/PlotBranchingSystem/Blueprint/Component/AC_PlotInteraction_Component.AC_PlotInteraction_Component_C|GetGet%20Target (Variables|Default|Get%20Plot%20Interaction))
                  (Variables|/Game/PlotBranchingSystem/Blueprint/Component/AC_PlotInteraction_Component.AC_PlotInteraction_Component_C|SetIn%20the%20plot (Variables|Default|Get%20Plot%20Interaction) true)
                  (goto _label))))))))))

(event OnComponentEndOverlap(Box)
  (params (OverlappedComponent :type Primitive%20Component%20Object%20Reference) (OtherActor :type Actor%20Object%20Reference) (OtherComp :type Primitive%20Component%20Object%20Reference) (OtherBodyIndex :type Integer))
  ;[1 1 1] 离开触发器
)

(event Custom|Event_Open%20Guidance
  (bind _returnvalue (UserInterface|CreateWidget "/Game/PlotBranchingSystem/UI/UI_Target.UI_Target_C" 0 self))
  (bind _output_get (Variables|Default|SetUI_Target _returnvalue))
  (UserInterface|Viewport|AddtoViewport _output_get 0))

(event Custom|Event_Set%20Target%20Display
  (params (IsDisplay :type Boolean))
  ;[1 0.2741 0] 设置目标点可视性
  (Rendering|SetVisibility (Variables|Default|GetTextRender) IsDisplay IsDisplay))

(event Custom|Event_Close%20Guidance
  (bind _ui_target (Variables|Default|GetUI_Target))
  (Utilities|IsValid _ui_target
    (:Is%20Valid
      (Default|UIEventCloseGuidance _ui_target))))

(event Custom|Event_Play%20Transition%20Sequences
  (params (Random%20Play :type Boolean) (Dimension%201 :type Integer))
  (bind _plot_data (Variables|Default|GetPlot_Data))
  (bind _transition_animation_sequence (Variables|/Game/PlotBranchingSystem/Data/PDA_Plot_Data.PDA_Plot_Data_C|GetTransition%20animation%20sequence _plot_data))
  (bind _output (Utilities|Array|Get(acopy) _transition_animation_sequence Dimension%201))
  ;[1 0.2741 0] 播放过场序列
  (Utilities|IsValid _output
    (:Is%20Valid
      (Utilities|IsValid (Variables|Default|GetOut%20Actor)
        (:Is%20Valid
          (Actor|DestroyActor (Variables|Default|GetOut%20Actor)))
        (:Is%20Not%20Valid
          _))
      (bind _outactor (Sequencer|Player|CreateLevelSequencePlayer _output))
      (bind _output_get (Variables|Default|SetOut%20Actor _outactor))
      (Sequencer|Player|Play (Variables|/Script/LevelSequence.LevelSequenceActor|GetSequencePlayer _output_get) :!class /Script/MovieScene.MovieSceneSequencePlayer))))

(event Custom|Event_Set%20Enable%20trigger
  (params (NewType :type ECollisionEnabled%20Enum :default "NoCollision"))
  (Collision|SetCollisionEnabled (Variables|Default|GetBox) NewType))

(event EventBeginPlay
  ;[0 0.7967 1] 获取玩家以及剧情交互组件
  (bind _asbp_third_person_character (Utilities|Casting|CastToBP_ThirdPersonCharacter (Game|Player|GetPlayerPawn 0)))
  (Variables|Default|SetPlayer _asbp_third_person_character)
  (Variables|Default|Set%20Plot%20Interaction (Variables|/Game/ThirdPerson/Blueprints/BP_ThirdPersonCharacter.BP_ThirdPersonCharacter_C|GetAC_PlotInteraction_Component _asbp_third_person_character))
  (Rendering|SetVisibility (Variables|Default|GetTextRender) false false)
  (if (Variables|条件|GetDefault%20Open%20Guide)
    (CallFunction|EventOpenGuidance)))

(event EventPlaySequence
  (CallFunction|EventPlayTransitionSequences false (Variables|/Game/PlotBranchingSystem/Blueprint/Component/AC_PlotInteraction_Component.AC_PlotInteraction_Component_C|GetCurrent%20number (Variables|Default|Get%20Plot%20Interaction))))

(event EventInteractive
  ;[1 1 1] 交互
  (Variables|/Game/PlotBranchingSystem/Blueprint/Component/AC_PlotInteraction_Component.AC_PlotInteraction_Component_C|SetIn%20the%20plot (Variables|Default|Get%20Plot%20Interaction) true)
  (CallFunction|TriggerthePlot (Variables|Default|GetPlot_Data))
  (CallFunction|EventCloseGuidance)
  (Utilities|IsValid (Variables|条件|Getlook%20at%20actor)
    (:Is%20Valid
      (Transformation|SetActorRotation (Variables|Default|GetPlayer) (Math|Rotator|MakeRotator 0.0 0.0 (.yaw (Math|Rotator|FindLookatRotation (Transformation|GetActorLocation (Variables|Default|GetPlayer)) (Transformation|GetActorLocation (Variables|条件|Getlook%20at%20actor)))))))))

(fn ConstructionScript
  (bind _box (Variables|Default|GetBox))
  (bind _returnvalue (Transformation|GetRelativeTransform _box))
  (Utilities|FlowControl|Sequence
    (:then_0
      (Rendering|Components|TextRender|SetText (Variables|Default|GetTextRender) (Variables|Default|GetScene%20display%20text)))
    (:then_1
      (CallFunction|EventSetEnableTrigger (Variables|条件|GetDefault%20trigger%20settings)))
    (:then_2
      (Transformation|SetRelativeTransform (Variables|Default|GetBox) (Math|Transform|MakeTransform (.location _returnvalue) (.rotation _returnvalue) (Variables|条件|GetTrigger%20box%20size)) false false))
    (:then_3
      (if (Variables|条件|GetUsing%20triggers%20)
        (Variables|条件|SetFor%20interactive%20objects false)))
    (:then_4
      (if (Variables|条件|GetFor%20interactive%20objects)
        (Variables|条件|SetUsing%20triggers%20 false)))))

(fn TriggerthePlot
  (params (Data :type PDA%20Plot%20Data%20Object%20Reference))
  (Utilities|FlowControl|Sequence
    (:then_1
      (Default|ACEventPloteStart (Variables|Default|Get%20Plot%20Interaction) (Variables|条件|GetRestrict%20Player%20Movement) (Variables|条件|GetRestrict%20Player%20Perspective) Data))))